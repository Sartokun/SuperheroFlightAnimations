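; BP_Dummy is a training dummy character that reacts to hits with a random montage, a pitched sound and a launch along the player's facing.
; BPCPlayerStats tracks health, a looping timer regenerates it, and the health bar widget turns toward the camera.
; On death it ragdolls, clears the player's SuperheroFlightComponent target lock and swaps its tags, then after a delay restores health, mesh, bar and regeneration.
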(event Custom|Ragdoll
  ;[0.05098 0.05098 0.05098] Ragdoll
  (Utilities|FlowControl|Delay 2.5)
  (Physics|SetSimulatePhysics (Variables|Character|GetMesh) true))

(event EventTick
  (params (DeltaSeconds :type Float%20%28single-precision%29))
  (Transformation|SetWorldRotation (Variables|Default|GetHealth%20Bar%20Widget) (Math|Rotator|FindLookatRotation (Transformation|GetWorldLocation (Variables|Default|GetHealth%20Bar%20Widget)) (Transformation|GetWorldLocation (Variables|/Script/Engine.PlayerCameraManager|GetTransformComponent (Game|GetPlayerCameraManager 0)))) false false))

(event Game|Damage|EventAnyDamage
  (params (Damage :type Float%20%28single-precision%29) (DamageType :type Damage%20Type%20Object%20Reference) (InstigatedBy :type Controller%20Object%20Reference) (DamageCauser :type Actor%20Object%20Reference))
  (bind _mesh (Variables|Character|GetMesh))
  (bind _mesh_2 (Variables|Character|GetMesh))
  (bind _returnvalue (Components|GetOwner _mesh))
  (Animation|PlayAnimMontage (Utilities|Array|Get(acopy) (Variables|Default|GethitAnims) (Math|Random|RandomIntegerinRange 0 (- (Utilities|Array|Length (Variables|Default|GethitAnims)) 1))) 1.0 "None")
  (bind _asbp_player_ue5 (Utilities|Casting|CastToBP_Player_UE5 (Game|GetPlayerCharacter 0)))
  (Character|LaunchCharacter (* (Math|Vector|GetForwardVector (Transformation|GetActorRotation _asbp_player_ue5)) 1e+03) false false)
  (Audio|PlaySoundatLocation "/Game/SuperheroFlight/Audio/Sword_Hits/Hit.Hit" (Transformation|GetActorLocation) "0, 0, 0" 1.0 (Math|Random|RandomFloatinRange 1.5 3.0) 0.0 "/Game/SuperheroFlight/Audio/SA_Character.SA_Character" 0 0 0)
  (bind _is_player_dead_ (Default|DecreaseHealth (Variables|Default|GetBPC_PlayerStats) Damage))
  (if _is_player_dead_
    (Physics|SetSimulatePhysics (Variables|Character|GetMesh) true)
    (Rendering|SetVisibility (Variables|Default|GetHealth%20Bar%20Widget) false false)
    (Utilities|Time|PauseTimerbyHandle (Variables|Default|GetTimer_IncreaseHealth))
    (bind _asbp_player_ue5_2 (Utilities|Casting|CastToBP_Player_UE5 (Game|GetPlayerCharacter 0)))
    (Variables|/Game/SuperheroFlight/Blueprints/Components/BP_SuperheroFlightComponent.BP_SuperheroFlightComponent_C|SetTaget? (Variables|/Game/SuperheroFlight/Blueprints/Characters/BP_Player_UE5.BP_Player_UE5_C|GetSuperheroFlightComponent _asbp_player_ue5_2) false)
    (Variables|/Game/SuperheroFlight/Blueprints/Components/BP_SuperheroFlightComponent.BP_SuperheroFlightComponent_C|SetactorToTargetLock (Variables|/Game/SuperheroFlight/Blueprints/Characters/BP_Player_UE5.BP_Player_UE5_C|GetSuperheroFlightComponent _asbp_player_ue5_2) 0)
    (Default|SetIsAimingFunc (Variables|/Game/SuperheroFlight/Blueprints/Characters/BP_Player_UE5.BP_Player_UE5_C|GetSuperheroFlightComponent _asbp_player_ue5_2) false)
    (Default|AutoTargetLock (Variables|/Game/SuperheroFlight/Blueprints/Characters/BP_Player_UE5.BP_Player_UE5_C|GetSuperheroFlightComponent _asbp_player_ue5_2) _returnvalue)
    (Variables|/Script/Engine.Actor|SetTags _returnvalue (Variables|Default|GetTags_0))
    (Utilities|FlowControl|Delay 5.0)
    (Physics|SetSimulatePhysics (Variables|Character|GetMesh) false)
    (Variables|/Game/SuperheroFlight/Blueprints/Characters/BPC_PlayerStats.BPC_PlayerStats_C|SetCurrent%20Health (Variables|Default|GetBPC_PlayerStats) 1e+02)
    (Rendering|SetVisibility (Variables|Default|GetHealth%20Bar%20Widget) true false)
    (Utilities|Time|UnpauseTimerbyHandle (Variables|Default|GetTimer_IncreaseHealth))
    (Variables|/Script/Engine.Actor|SetTags _returnvalue (Variables|Default|GetTags_1))
    (Transformation|SetWorldRotation _mesh_2 "0.000000,-90.000000,0.000000" false false)
    (Transformation|SetWorldLocation _mesh_2 (- (Transformation|GetWorldLocation (Variables|Collision|GetCapsuleComponent)) "0.000000,0.000000,89.000000") false true)))

(event EventBeginPlay
  (Utilities|FlowControl|Sequence
    (:then_0
      (bind _aswb_dummy_health (Utilities|Casting|CastToWB_DummyHealth (UserInterface|GetWidget (Variables|Default|GetHealth%20Bar%20Widget))))
      (Variables|Default|SetHealth%20Bar%20Ui _aswb_dummy_health))
    (:then_1
      (bind _returnvalue (Utilities|Time|SetTimerbyFunctionName 0 "Increase Health" 5.0 true))
      (Variables|Default|SetTimer_IncreaseHealth _returnvalue))))

(fn ConstructionScript)

(fn IncreaseHealth
  (Default|IncreaseHealth (Variables|Default|GetBPC_PlayerStats) 5.0))