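; Actor component that tracks health and energy, detecting at BeginPlay whether its owner is the player or a dummy.
; Health functions apply damage, capped healing and max increases, then refresh a bar and text, with only the dummy's widget wired as target.
; DecreaseHealth returns whether health is depleted.
; Energy drains and regenerates by set amounts within clamped limits, while AddEnergy adds without clamping and CheckEnergy flags depletion.
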(event EventBeginPlay
  (bind _returnvalue (Components|GetOwner))
  (Utilities|FlowControl|DelayUntilNextTick)
  (bind _asbp_player_ue5 (Utilities|Casting|CastToBP_Player_UE5 _returnvalue)
    (:then
      (Variables|Default|SetPlayer%20Character%20BP _asbp_player_ue5)
      (Variables|Default|SetisPlayer? true))
    (:CastFailed
      (bind _asbp_dummy (Utilities|Casting|CastToBP_Dummy _returnvalue))
      (Variables|Default|SetDummy%20BP _asbp_dummy)
      (Variables|Default|SetisPlayer? false)
      (Progress|SetPercent (select (Variables|Default|GetisPlayer?) 0 (Variables|/Game/SuperheroFlight/UI/WB_DummyHealth.WB_DummyHealth_C|GetHealthBar (Variables|/Game/SuperheroFlight/Blueprints/BP_Dummy.BP_Dummy_C|GetHealth%20Bar%20Ui (Variables|Default|GetDummy%20BP)))) (/ (Variables|Health|GetCurrent%20Health) (Variables|Health|GetMax%20Health)))
      (Rendering|Components|TextRender|SetText (select (Variables|Default|GetisPlayer?) 0 (Variables|/Game/SuperheroFlight/UI/WB_DummyHealth.WB_DummyHealth_C|GetHealthText (Variables|/Game/SuperheroFlight/Blueprints/BP_Dummy.BP_Dummy_C|GetHealth%20Bar%20Ui (Variables|Default|GetDummy%20BP)))) (Utilities|Text|ToText(Float) (Variables|Health|GetCurrent%20Health) "HalfToEven")))))

(fn DecreaseHealth
  (params (Damage :type Float%20%28double-precision%29))
  (Variables|Health|SetCurrent%20Health (- (Variables|Health|GetCurrent%20Health) Damage))
  (Progress|SetPercent (select (Variables|Default|GetisPlayer?) 0 (Variables|/Game/SuperheroFlight/UI/WB_DummyHealth.WB_DummyHealth_C|GetHealthBar (Variables|/Game/SuperheroFlight/Blueprints/BP_Dummy.BP_Dummy_C|GetHealth%20Bar%20Ui (Variables|Default|GetDummy%20BP)))) (/ (Variables|Health|GetCurrent%20Health) (Variables|Health|GetMax%20Health)))
  (Rendering|Components|TextRender|SetText (select (Variables|Default|GetisPlayer?) 0 (Variables|/Game/SuperheroFlight/UI/WB_DummyHealth.WB_DummyHealth_C|GetHealthText (Variables|/Game/SuperheroFlight/Blueprints/BP_Dummy.BP_Dummy_C|GetHealth%20Bar%20Ui (Variables|Default|GetDummy%20BP)))) (Utilities|Text|ToText(Float) (Variables|Health|GetCurrent%20Health) "HalfToEven"))
  (if (<= (Variables|Health|GetCurrent%20Health) 0.0)
    (return true)
    (else
      (return false))))

(fn IncreaseMaxHealth
  (params (Health%20Incremention :type Float%20%28double-precision%29))
  (Variables|Health|SetMax%20Health (+ Health%20Incremention (Variables|Health|GetMax%20Health)))
  (Progress|SetPercent (select (Variables|Default|GetisPlayer?) 0 (Variables|/Game/SuperheroFlight/UI/WB_DummyHealth.WB_DummyHealth_C|GetHealthBar (Variables|/Game/SuperheroFlight/Blueprints/BP_Dummy.BP_Dummy_C|GetHealth%20Bar%20Ui (Variables|Default|GetDummy%20BP)))) (/ (Variables|Health|GetCurrent%20Health) (Variables|Health|GetMax%20Health)))
  (Rendering|Components|TextRender|SetText (select (Variables|Default|GetisPlayer?) 0 (Variables|/Game/SuperheroFlight/UI/WB_DummyHealth.WB_DummyHealth_C|GetHealthText (Variables|/Game/SuperheroFlight/Blueprints/BP_Dummy.BP_Dummy_C|GetHealth%20Bar%20Ui (Variables|Default|GetDummy%20BP)))) (Utilities|Text|ToText(Float) (Variables|Health|GetCurrent%20Health) "HalfToEven")))

(fn IncreaseHealth
  (params (Added%20Health :type Float%20%28double-precision%29))
  (Variables|Health|SetCurrent%20Health (+ Added%20Health (Variables|Health|GetCurrent%20Health)))
  (if (> (Variables|Health|GetCurrent%20Health) (Variables|Health|GetMax%20Health))
    (Variables|Health|SetCurrent%20Health (Variables|Health|GetMax%20Health)))
  (Progress|SetPercent (select (Variables|Default|GetisPlayer?) 0 (Variables|/Game/SuperheroFlight/UI/WB_DummyHealth.WB_DummyHealth_C|GetHealthBar (Variables|/Game/SuperheroFlight/Blueprints/BP_Dummy.BP_Dummy_C|GetHealth%20Bar%20Ui (Variables|Default|GetDummy%20BP)))) (/ (Variables|Health|GetCurrent%20Health) (Variables|Health|GetMax%20Health)))
  (Rendering|Components|TextRender|SetText (select (Variables|Default|GetisPlayer?) 0 (Variables|/Game/SuperheroFlight/UI/WB_DummyHealth.WB_DummyHealth_C|GetHealthText (Variables|/Game/SuperheroFlight/Blueprints/BP_Dummy.BP_Dummy_C|GetHealth%20Bar%20Ui (Variables|Default|GetDummy%20BP)))) (Utilities|Text|ToText(Float) (Variables|Health|GetCurrent%20Health) "HalfToEven")))

(fn GetHealth
  (return (Variables|Health|GetCurrent%20Health)))

(fn DecreaseEnergy
  (Variables|Energy|SetCurrentEnergy (Math|Float|Clamp(Float) (- (Variables|Energy|GetCurrentEnergy) (Variables|Energy|GetUsageEnergy)) 0.0 (Variables|Energy|GetMaxEnergy))))

(fn IncreaseEnergy
  (Variables|Energy|SetCurrentEnergy (Math|Float|Clamp(Float) (+ (Variables|Energy|GetCurrentEnergy) (Variables|Energy|GetRegenerationEnergy)) 0.0 (Variables|Energy|GetMaxEnergy))))

(fn CheckEnergy
  (if (> (Variables|Energy|GetCurrentEnergy) 0.0)
    (Variables|Energy|SetCheck_Energy true)
    (else
      (Variables|Energy|SetCheck_Energy false)))
  (if (not (Variables|Energy|GetCheck_Energy))
    (Development|PrintString "Energy <= 0")))

(fn GetCurrentEnergy
  (return (Variables|Energy|GetCurrentEnergy)))

(fn AddEnergy
  (params (Energy :type Float%20%28double-precision%29))
  (Variables|Energy|SetCurrentEnergy (+ Energy (Variables|Energy|GetCurrentEnergy))))